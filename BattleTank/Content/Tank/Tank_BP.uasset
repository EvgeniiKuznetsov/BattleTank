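; Tank Blueprint that provides physics simulation and camera aiming controls.
; On BeginPlay it enables physics on the Tank component and passes the Barrel component to SetBarrelReference.
; The AimAzimuth axis yaws the AzimuthGimbal and the AimAlimus axis pitches the SpringArm, both as local rotations scaled by delta time for frame-rate independence.
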(event `self.ReceiveBeginPlay`
  (`PrimitiveComponent.SetSimulatePhysics` (`self.Tank`) true)
  (`self.SetBarrelReference` (`self.Barrel`)))

(event `InputAxis|AimAzimuth`
  (params (AxisValue :type "Float (single-precision)"))
  (`SceneComponent.K2_AddLocalRotation` (`self.Azimuth Gimbal`) (`KismetMathLibrary.MakeRotator` 0.0 0.0 (* AxisValue (`GameplayStatics.GetWorldDeltaSeconds`) 100.0)) false false))

(event `InputAxis|AimAlimus`
  (params (AxisValue :type "Float (single-precision)"))
  (`SceneComponent.K2_AddLocalRotation` (`self.SpringArm`) (`KismetMathLibrary.MakeRotator` 0.0 (* AxisValue (`GameplayStatics.GetWorldDeltaSeconds`) 100.0)) false false))

(fn `UserConstructionScript`)